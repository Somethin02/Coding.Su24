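; BP_Key is a collectible key pickup that increments the player's key count.
; When its BoxCollision is overlapped, it casts the other actor to BP_ThirdPersonCharacterCustom, adds one to that character's KeyCount and destroys itself.
; Debug strings print on BeginPlay, on pickup with the new count, and when the cast fails for other overlapping actors.
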(event `self.ReceiveBeginPlay`
  (`KismetSystemLibrary.PrintString` "This Key exists!" true true (struct :`R` 1.0 :`B` 0.987577 :`A` 1.0)))

(event `self. Box Collision.OnComponentBeginOverlap`
  (params (OverlappedComponent :type "PrimitiveComponent Object Reference") (OtherActor :type "Actor Object Reference") (OtherComp :type "PrimitiveComponent Object Reference") (OtherBodyIndex :type Integer) (bFromSweep :type Boolean) (SweepResult :type "HitResult Structure (by ref)"))
  (bind _asbp_third_person_character_custom (cast `/Game/Blueprints/BP_ThirdPersonCharacterCustom` OtherActor)
    (:`then`
      (`KismetSystemLibrary.PrintString` "Key has been overlapped by player!" true true (struct :`G` 0.66 :`B` 1.0 :`A` 1.0) 5.0)
      (bind _key_count (`/Game/Blueprints/BP_ThirdPersonCharacterCustom.key Count` _asbp_third_person_character_custom))
      (set `/Game/Blueprints/BP_ThirdPersonCharacterCustom.key Count` (+ _key_count 1) _asbp_third_person_character_custom)
      (`KismetSystemLibrary.PrintString` (`KismetStringLibrary.Concat_StrStr` "The player has " (`KismetStringLibrary.Conv_IntToString` _key_count) " key(s)"))
      (`self.K2_DestroyActor`))
    (:`CastFailed`
      (`KismetSystemLibrary.PrintString` "Key Player Type cast failed!" true true (struct :`R` 1.0 :`G` 0.050762 :`B` 0.170476 :`A` 1.0)))))

(fn `UserConstructionScript`)