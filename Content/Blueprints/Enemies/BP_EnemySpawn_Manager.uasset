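; Enemy spawn manager that runs endless waves of BP_Enemy from the BP_EnemySpawner actors in the level.
; On BeginPlay it caches every spawner and spawns one enemy at each spawner's transform, giving each a reference back to the manager.
; RemoveEnemyandCheck decrements the live count and, when it reaches zero, announces a new wave and respawns after a short delay.
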(event `self.ReceiveBeginPlay`
  (`KismetSystemLibrary.PrintString` "Enemy Spawn Manager is ready!")
  (bind _outactors (`GameplayStatics.GetAllActorsOfClass` "/Game/Blueprints/Enemies/BP_EnemySpawner.BP_EnemySpawner_C"))
  (set `self.Spawners` _outactors)
  (`self.Spawn Enemies`))

(event `Spawn Enemies`
  (for _array_element (`self.Spawners`)
    (bind (_returnvalue_location _returnvalue_rotation) (`KismetMathLibrary.BreakTransform` (`SceneComponent.K2_GetComponentToWorld` (`/Game/Blueprints/Enemies/BP_EnemySpawner.DefaultSceneRoot` _array_element))))
    (bind _returnvalue (`|SpawnActorFromClass` "/Game/Blueprints/Enemies/BP_Enemy.BP_Enemy_C" (`KismetMathLibrary.MakeTransform` _returnvalue_location _returnvalue_rotation) "Undefined" "MultiplyWithRoot" null null))
    (set `/Game/Blueprints/Enemies/BP_Enemy.Manager` self _returnvalue)
    (`/Engine/EditorBlueprintResources/StandardMacros.IncrementInt` (`self.CurrentEnemyTotal`))))

(event `Remove Enemy and Check`
  (`/Engine/EditorBlueprintResources/StandardMacros.DecrementInt` (`self.CurrentEnemyTotal`)
    (:`  `
      (if (not (> (`self.CurrentEnemyTotal`) 0))
        (`KismetSystemLibrary.PrintString` "New Wave Incoming" true true (struct :`G` 0.66 :`B` 1.0 :`A` 1.0) 5.0)
        (`KismetSystemLibrary.Delay` 5.0)
        (`self.Spawn Enemies`)))))

(fn `UserConstructionScript`)