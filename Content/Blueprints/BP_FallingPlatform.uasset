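; BP_FallingPlatform is a platform that drops shortly after the custom third-person character touches its collision, then returns to its start.
; On overlap, a Ready flag blocks retriggering while a one-second warning runs, after which physics simulation makes the platform fall.
; Three seconds later, physics turns off and a Timeline lerps it back to the transform saved at BeginPlay, re-arming it.
; Material swaps and debug prints mark each state.
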(event `self.ReceiveBeginPlay`
  (set `self.Starting Transform` (`SceneComponent.K2_GetComponentToWorld` (`self.Falling Platform`))))

(event `self.Collision.OnComponentBeginOverlap`
  (params (OverlappedComponent :type "PrimitiveComponent Object Reference") (OtherActor :type "Actor Object Reference") (OtherComp :type "PrimitiveComponent Object Reference") (OtherBodyIndex :type Integer) (bFromSweep :type Boolean) (SweepResult :type "HitResult Structure (by ref)"))
  (cast `/Game/Blueprints/BP_ThirdPersonCharacterCustom` OtherActor)
  (`self.Activate`))

(event `Activate`
  (if (`self.Ready`)
    (`KismetSystemLibrary.PrintString` "One second left!")
    (set `self.Ready` false)
    (`PrimitiveComponent.SetMaterial` (`self.Falling Platform`) 0 "/Game/Materials/Mi_Platform_Danger.Mi_Platform_Danger")
    (`KismetSystemLibrary.Delay` 1.0)
    (`self.Drop`)))

(event `Drop`
  (`KismetSystemLibrary.PrintString` "Down we go!")
  (`PrimitiveComponent.SetSimulatePhysics` (`self.Falling Platform`) true)
  (`PrimitiveComponent.SetMaterial` (`self.Falling Platform`) 0 "/Game/Materials/Mi_Platform_Falling.Mi_Platform_Falling")
  (`KismetSystemLibrary.Delay` 3.0)
  (`self.Reset`))

(event `Reset`
  (`KismetSystemLibrary.PrintString` "Resetting")
  (set `self.Reset Transform` (`SceneComponent.K2_GetComponentToWorld` (`self.Falling Platform`)))
  (`PrimitiveComponent.SetSimulatePhysics` (`self.Falling Platform`) false)
  (`PrimitiveComponent.SetMaterial` (`self.Falling Platform`) 0 "/Game/Materials/Mi_Platform_Reset.Mi_Platform_Reset")
  (bind (_direction _newtrack_0) (`Timeline|Timeline` :!via `PlayFromStart`)
    (:`Update`
      (bind (_returnvalue_location _returnvalue_rotation) (`KismetMathLibrary.BreakTransform` (`KismetMathLibrary.TLerp` (`self.Reset Transform`) (`self.Starting Transform`) _newtrack_0)))
      (`SceneComponent.K2_SetWorldLocationAndRotation` (`self.Falling Platform`) _returnvalue_location _returnvalue_rotation false false))
    (:`Finished`
      (set `self.Ready` true)
      (`PrimitiveComponent.SetMaterial` (`self.Falling Platform`) 0 "/Game/Materials/Mi_Platform_Ready.Mi_Platform_Ready"))))

(fn `UserConstructionScript`)