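; BP_LoopsAndLists is a demonstration actor for loop and array techniques, reporting through on-screen prints.
; BeginPlay starts two endless Delay-paced loops, a simple print and a self-calling counter that periodically resets, then gathers all BP_Key actors.
; ChangeKeyColor repeatedly tints one key at a time via dynamic material instances, shuffling keys and colors when exhausted and re-querying invalid keys.
; Input triggers a bounded while loop and string-array length, indexing and iteration examples.
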(event `self.ReceiveBeginPlay`
  (`KismetSystemLibrary.PrintString` "Loops and Lists are starting" true true (struct :`G` 0.66 :`B` 1.0 :`A` 1.0) 5.0)
  (`|ExecutionSequence`
    (:`then_0`
      ;[1 1 1] Set up for loops
      (`self.Simple Game Loop`)
      (`self.EnableInput` (`GameplayStatics.GetPlayerController` 0))
      (`self.Recursive loop`))
    (:`then_1`
      ;[1 1 1] Set up for lists
      (bind _outactors (`GameplayStatics.GetAllActorsOfClass` "/Game/Blueprints/BP_Key.BP_Key_C"))
      (set `self.Keys` _outactors)
      (`self.Change Key Color`))))

(event `Simple Game Loop`
  (`KismetSystemLibrary.PrintString` "Starting Game Loop" :!label _label)
  (`KismetSystemLibrary.Delay` 1.0)
  (goto _label))

(event `self.ReceiveTick`
  (params (DeltaSeconds :type "Float (single-precision)")))

(event `InputAction|start While Loop`
  (params (Key :type "Key Structure"))
  (bind _while_loop_counter (`self.While loop counter`))
  (:`Pressed`
    (`KismetSystemLibrary.PrintString` "Starting While Loop")
    (while (< (`self.While loop counter`) 25)
      (`/Engine/EditorBlueprintResources/StandardMacros.IncrementInt` _while_loop_counter
        (:`  `
          (`KismetSystemLibrary.PrintString` (`KismetStringLibrary.Concat_StrStr` "This While Loop has run " (`KismetStringLibrary.Conv_IntToString` _while_loop_counter) " times.") true true (`KismetMathLibrary.MakeColor` (`KismetMathLibrary.RandomFloat`) (`KismetMathLibrary.RandomFloat`) (`KismetMathLibrary.RandomFloat`))))))
    (`KismetSystemLibrary.PrintString` "The While Loop is complete.")
    (set `self.While loop counter` 0)))

(event `Recursive loop`
  (if (< (`self.Recursion Counter`) 5)
    (bind _result (`/Engine/EditorBlueprintResources/StandardMacros.IncrementInt` (`self.Recursion Counter`))
      (:`  `
        (`KismetSystemLibrary.PrintString` (`KismetStringLibrary.Concat_StrStr` "The recursive Loop has run " (`KismetStringLibrary.Conv_IntToString` _result) " times.") true true (struct :`R` 1.0 :`G` 0.444173 :`B` 0.769146 :`A` 1.0) 1.2)
        (`KismetSystemLibrary.Delay` 1.0)))
    (else
      (`KismetSystemLibrary.PrintString` "Resetting recursive loop")
      (set `self.Recursion Counter` 0)
      (`KismetSystemLibrary.Delay` 3.0)))
  (`self.Recursive loop`))

(event `Key|Six`
  (params (Key :type "Key Structure"))
  (:`Pressed`
    (`self.First Array Test`)))

(event `First Array Test`
  (bind _array (`|MakeArray` "Mario" "Luigi" "Toad" "Yoshi"))
  (`KismetSystemLibrary.PrintString` (`KismetStringLibrary.Concat_StrStr` "Our array of strings has " (`KismetStringLibrary.Conv_IntToString` (`KismetArrayLibrary.Array_Length` _array)) " names in it."))
  (`KismetSystemLibrary.PrintString` (`KismetStringLibrary.Concat_StrStr` "The first name in the array is " (`|GetArrayItem` _array) ".")))

(event `Key|Five`
  (params (Key :type "Key Structure"))
  (:`Pressed`
    (`self.Display Entire array`)))

(event `Display Entire array`
  (for (_array_element _array_index) (`|MakeArray` "Mario" "Luigi" "Toad" "Yoshi")
    (`KismetSystemLibrary.PrintString` (`KismetStringLibrary.Concat_StrStr` (`KismetStringLibrary.Conv_IntToString` (+ _array_index 1)) ". " _array_element) true true (struct :`R` 0.226388 :`G` 0.316291 :`B` 1.0 :`A` 1.0))))

(event `Change Key Color`
  (bind _keys (`self.Keys`))
  (bind _output (`|GetArrayItem` _keys (`self.Color Key index`)))
  (if (or (>= (`self.Color Key index`) (`KismetArrayLibrary.Array_Length` (`self.Color`))) (>= (`self.Color Key index`) (`KismetArrayLibrary.Array_Length` (`self.Keys`))))
    ;[1 1 1] Shuffle and reset
    (`KismetArrayLibrary.Array_Shuffle` (`self.Color`))
    (`KismetArrayLibrary.Array_Shuffle` _keys)
    (set `self.Color Key index` 0))
  (`/Engine/EditorBlueprintResources/StandardMacros.IsValid` _output
    (:`Is Valid`
      ;[1 1 1] Setting the color
      (bind _returnvalue (`PrimitiveComponent.CreateDynamicMaterialInstance` (`/Game/Blueprints/BP_Key.Cylinder` _output) 0 "/Game/Materials/M_Base.M_Base" "None"))
      (`MaterialInstanceDynamic.SetVectorParameterValue` _returnvalue "Base Color" (`KismetMathLibrary.Conv_ColorToLinearColor` (`|GetArrayItem` (`self.Color`) (`self.Color Key index`)))))
    (:`Is Not Valid`
      (bind _outactors (`GameplayStatics.GetAllActorsOfClass` "/Game/Blueprints/BP_Key.BP_Key_C")) ; If a key is missing look for all keys and reset the array of keys
      (set `self.Keys` _outactors)))
  (`/Engine/EditorBlueprintResources/StandardMacros.IncrementInt` (`self.Color Key index`)
    (:`  `
      (`KismetSystemLibrary.Delay` 0.5)
      (`self.Change Key Color`))))

(fn `UserConstructionScript`)